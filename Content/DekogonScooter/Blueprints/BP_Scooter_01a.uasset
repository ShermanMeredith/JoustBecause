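; BP_Scooter_01a is a drivable scooter vehicle with throttle, steering, handbrake, camera look, horns and lights.
; Input drives the vehicle movement component, toggles the headlight and lights the stop light on reverse throttle or handbrake.
; Tick eases steering into the anim Blueprint's handlebar and root rotations, and feeds forward speed and horn states to audio parameters.
; The construction script applies configurable body material, light colors and intensities, matching emissive material parameters to the lights.
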(event EventBeginPlay
  (bind _asabp_scooter_01a (Utilities|Casting|CastToABP_Scooter_01a (Components|SkeletalMesh|GetAnimInstance (Variables|Character|GetMesh))))
  (Variables|Default|SetABP_Scooter _asabp_scooter_01a))

(event EventTick
  (params (DeltaSeconds :type Float%20%28single-precision%29))
  (bind _abp_scooter (Variables|Default|GetABP_Scooter))
  (bind _sc_honks (Variables|Default|GetSC_Honks))
  (bind _vehiclemovement (Variables|Default|GetVehicleMovement))
  (bind _vehiclerpm (Variables|Default|GetVehicleRPM))
  (bind _returnvalue (Class|WheeledVehicleMovementComponent|GetForwardSpeed _vehiclemovement))
  (bind _returnvalue_2 (Math|Float|Absolute(Float) _returnvalue))
  ;[1 1 1] Wheel Handler
  (Variables|/Game/DekogonScooter/Blueprints/ABP_Scooter_01a.ABP_Scooter_01a_C|SetHandlerRotation _abp_scooter (Math|Interpolation|FInterpTo (Variables|/Game/DekogonScooter/Blueprints/ABP_Scooter_01a.ABP_Scooter_01a_C|GetHandlerRotation _abp_scooter) (* 15.0 (Input|AxisValues|GetSteer)) (Utilities|Time|GetWorldDeltaSeconds) 3.0))
  (Variables|/Game/DekogonScooter/Blueprints/ABP_Scooter_01a.ABP_Scooter_01a_C|SetRoot _abp_scooter (Math|Interpolation|FInterpTo (Variables|/Game/DekogonScooter/Blueprints/ABP_Scooter_01a.ABP_Scooter_01a_C|GetRoot _abp_scooter) (* 7.0 (Input|AxisValues|GetSteer)) (Utilities|Time|GetWorldDeltaSeconds) 3.0))
  ;[1 1 1] Audio
  (Audio|Parameter|SetFloatParameter _vehiclerpm "RPM" _returnvalue_2 :!class /Script/Engine.AudioComponent)
  (Audio|Components|Audio|SetPitchMultiplier _vehiclerpm (* (+ (/ _returnvalue_2 9e+03) 0.2) 1.4))
  (Effects|Components|ParticleSystem|SetBoolParameter _sc_honks "LongHonk" (Variables|Default|GetLongHonk))
  (Effects|Components|ParticleSystem|SetBoolParameter _sc_honks "ShortHonk" (Variables|Default|GetShortHonk)))

(event Input|AxisEvents|InputAxisThrottle
  (params (AxisValue :type Float%20%28single-precision%29))
  (bind _stoplight (Variables|Default|GetStopLight))
  ;[1 1 1] Vehicle Movement
  (Class|WheeledVehicleMovementComponent|SetThrottleInput (Variables|Default|GetVehicleMovement) AxisValue)
  ;[1 1 1] Stop Light
  (Math|Float|CompareFloat (Math|Conversions|ToFloat(Integer) (Class|KismetMathLibrary|OrIntInt (Math|Float|Truncate (* AxisValue -1.0)) (Math|Conversions|ToInteger(Boolean) (Variables|Default|GetBackLight)))) 1.0
    (:==
      (Rendering|Components|Light|SetIntensity _stoplight 4e+02))
    (:<
      (Rendering|Components|Light|SetIntensity _stoplight 0.0))))

(event Input|AxisEvents|InputAxisSteer
  (params (AxisValue :type Float%20%28single-precision%29))
  ;[1 1 1] Vehicle Movement
  (Class|WheeledVehicleMovementComponent|SetSteeringInput (Variables|Default|GetVehicleMovement) AxisValue))

(event Input|AxisEvents|InputAxisLookUp
  (params (AxisValue :type Float%20%28single-precision%29))
  ;[1 1 1] Vehicle Movement
  (Transformation|AddRelativeRotation (Variables|Default|GetSpringArm) (Math|Rotator|MakeRotator 0.0 AxisValue (stale Input|AxisEvents|InputAxisLookRight AxisValue)) false false))

(event Input|AxisEvents|InputAxisLookRight
  (params (AxisValue :type Float%20%28single-precision%29))
  ;[1 1 1] Vehicle Movement
  (Transformation|AddRelativeRotation (Variables|Default|GetSpringArm) (Math|Rotator|MakeRotator 0.0 (stale Input|AxisEvents|InputAxisLookUp AxisValue) AxisValue) false false))

(event Input|KeyboardEvents|H
  (params (Key :type Key%20Structure))
  ;[1 1 1] Horns
  (:Pressed
    (Variables|Default|SetShortHonk true))
  (:Released
    (Variables|Default|SetShortHonk false)))

(event Input|KeyboardEvents|G
  (params (Key :type Key%20Structure))
  ;[1 1 1] Horns
  (:Pressed
    (Variables|Default|SetLongHonk true))
  (:Released
    (Variables|Default|SetLongHonk false)))

(event Input|KeyboardEvents|J
  (params (Key :type Key%20Structure))
  (:Pressed
    (bind _isa (Utilities|FlowControl|FlipFlop)
      (:A
        _)
      (:B
        _))
    (Rendering|Components|Light|SetIntensity (Variables|Default|GetFrontLight) (* (* (Math|Conversions|ToFloat(Boolean) _isa) (Variables|Material|GetLight%20Intensity)) 5e+02))))

(event Input|KeyboardEvents|SpaceBar
  (params (Key :type Key%20Structure))
  (bind _vehiclemovement (Variables|Default|GetVehicleMovement))
  ;[1 1 1] Vehicle Movement
  (:Pressed
    (Variables|Default|SetBackLight true)
    (Class|WheeledVehicleMovementComponent|SetHandbrakeInput _vehiclemovement true))
  (:Released
    (Variables|Default|SetBackLight false)
    (Class|WheeledVehicleMovementComponent|SetHandbrakeInput _vehiclemovement false)))

(fn ConstructionScript
  (bind _mesh (Variables|Character|GetMesh))
  (bind _frontlight (Variables|Default|GetFrontLight))
  (bind _scooter_lightcolor (Variables|Material|GetScooter%20LightColor))
  (bind _sidelamps (Variables|Material|GetSideLamps))
  (bind _sidelampsintensity (Variables|Material|GetSideLampsIntensity))
  (bind _material_light_intensity (Variables|Material|GetMaterial%20Light%20Intensity))
  ;[1 1 1] Material
  (Rendering|Material|SetMaterial (Variables|Character|GetMesh) 0 (Variables|Material|GetScooter%20Material))
  ;[1 1 1] Light Settings
  (Rendering|Components|Light|SetLightColor _frontlight _scooter_lightcolor true)
  (Rendering|Material|SetVectorParameterValueonMaterials (Variables|Character|GetMesh) "Emissive Color Multi 3" (Math|Conversions|ToVector(LinearColor) _scooter_lightcolor))
  (Rendering|Components|Light|SetIntensity _frontlight (* _material_light_intensity 5e+02))
  (Rendering|Material|SetScalarParameterValueonMaterials (Variables|Character|GetMesh) "FrontLightIntensity" _material_light_intensity)
  (Rendering|Material|SetVectorParameterValueonMaterials _mesh "Emissive Color Multi 2" (Math|Conversions|ToVector(LinearColor) _sidelamps))
  (Rendering|Material|SetScalarParameterValueonMaterials _mesh "SideLampsIntensity" (/ _sidelampsintensity 5.0))
  (Rendering|Components|Light|SetIntensity (Variables|Default|GetSideLights1) _sidelampsintensity)
  (Rendering|Components|Light|SetLightColor (Variables|Default|GetSideLights2) _sidelamps true))